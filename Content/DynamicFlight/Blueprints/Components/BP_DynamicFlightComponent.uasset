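; Character component that gives the player Hover and FastFlight modes, switching player mode between Statue and Human.
; Toggles change movement settings; FastFlight shrinks the capsule and traces for room before restoring it on exit.
; Tick eases rotation toward the camera, computes lean rates and applies decaying left/right dodge forces.
; Actor hits trigger a ground slam on hard landings, or drop FastFlight into Hover with a bounce off walls.
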(event `self.ReceiveBeginPlay`
  (bind _movementcomponent (`self.MovementComponent`))
  ;[0.599 1 0.6833] Save references to the character, its capsule component, and its movement component.
  (bind _ascharacter (cast `Character` (`self.GetOwner`)))
  (set `self.Character` _ascharacter)
  (set `self.MovementComponent` (`Character.CharacterMovement` _ascharacter))
  (bind _output_get (set `self.CapsuleComponent` (`Character.CapsuleComponent` _ascharacter)))
  ;[0.599 1 0.6833] Record starting capsule size. Used to check if there's enough room, and restore the original capsule height, when exiting FastFlight.
  (set `self.CapsuleHalfHeight` (`CapsuleComponent.GetUnscaledCapsuleHalfHeight` _output_get))
  (set `self.CapsuleRadius` (`CapsuleComponent.GetUnscaledCapsuleRadius` _output_get))
  ;[0.599 1 0.6833] Set defaults for certain flight properties.
  (set `CharacterMovementComponent.MaxAcceleration` (`self.DefaultAcceleration`) _movementcomponent)
  (set `CharacterMovementComponent.BrakingDecelerationFlying` 1400.0 _movementcomponent)
  ;[0.599 1 0.6833] If a Hit event triggers on the character, run a custom event here.
  (add `Actor.OnActorHit` (`self.Character`) (delegate `Hit`)))

(event `Hit`
  (params (SelfActor :type "Actor Object Reference") (OtherActor :type "Actor Object Reference") (NormalImpulse :type "Vector Structure") (Hit :type "HitResult Structure (by ref)"))
  (bind (_bblockinghit _binitialoverlap _time _distance _location _impactpoint _normal _impactnormal) (`GameplayStatics.BreakHitResult` Hit))
  (bind _fastflight (`self.FastFlight`))
  (bind _character (`self.Character`))
  (bind _returnvalue (`KismetMathLibrary.DegAcos` (`KismetMathLibrary.Dot_VectorVector` (`SceneComponent.GetForwardVector` (`self.CapsuleComponent`)) _impactnormal)))
  (if (or (and (> _returnvalue 100.0) _fastflight) (and (not _fastflight) (`KismetMathLibrary.NearlyEqual_FloatFloat` _returnvalue 90.0 1.0)))
    (if (>= (.z _impactnormal) 0.5)
      (if (`self.FastFlight`)
        (`self.ToggleFastFlight`)
        (if (not (`self.FastFlight`))
          (`self.TriggerGroundSlam` :!label _label)
          (`PlayerCharacter.PlayCameraShake` (cast `/Game/_Users/Players/Blueprints/BP_Player` (`self.Character`) :!pure true) (enumliteral `ECameraShakeType` "Landhing") :!label _label_2))
        (else
          (bind _returnvalue_2 (`PrimitiveComponent.GetPhysicsLinearVelocity` (`Character.CapsuleComponent` (`self.Character`)) "None"))
          (if (<= (.z _returnvalue_2) -1000.0)
            (goto _label))))
      (elif (`self.FastFlight`)
        (`self.ToggleHover`)
        (`|ExecutionSequence`
          (:`then_0`
            (goto _label_2))
          (:`then_1`
            (`KismetSystemLibrary.Delay` 0.0)
            (`Character.LaunchCharacter` _character (* _impactnormal (`self.BounceForce`)) false false)
            (`PlayerCharacter.StopMove` (cast `/Game/_Users/Players/Blueprints/BP_PlayerBase` (`self.Character`) :!pure true) 1.0)
            (`KismetSystemLibrary.Delay` 0.0)
            (`CharacterMovementComponent.SetMovementMode` (`Character.CharacterMovement` _character) "MOVE_Flying" 0)))))))

(event `self.ReceiveTick`
  (params (DeltaSeconds :type "Float (single-precision)"))
  ;[0.599 1 0.6833] Call the FlightUpdates event each tick to update flight behaviors (that aren't driven by Movement Input)
  (set `self.Delta` DeltaSeconds)
  (`self.FlightUpdates`))

(event `FlightUpdates`
  (bind _returnvalue (`PrimitiveComponent.GetPhysicsAngularVelocityInDegrees` (`self.CapsuleComponent`) "None"))
  (bind _returnvalue_2 (`SceneComponent.GetRightVector` (`self.CameraComponent`)))
  (bind (_returnvalue_roll _returnvalue_pitch _returnvalue_yaw) (`KismetMathLibrary.BreakRotator` (`SceneComponent.K2_GetComponentRotation` (`self.CapsuleComponent`))))
  (bind _returnvalue_3 (`SceneComponent.K2_GetComponentRotation` (`self.CameraComponent`)))
  ;[0.599 1 0.6833] Updates flight logic if either flight mode is active.
  (if (or (`self.Hover`) (`self.FastFlight`))
    (`Actor.K2_SetActorRotation` (`self.Character`) (`KismetMathLibrary.RInterpTo` (`SceneComponent.K2_GetComponentRotation` (`self.CapsuleComponent`)) (select `bool` (`self.Hover`) :`false` _returnvalue_3 :`true` (`KismetMathLibrary.MakeRotator` (.roll _returnvalue_3) 0.0 (.yaw _returnvalue_3))) (`self.Delta`) 8.0) false)
    (set `self.X-RotationRate` (`KismetMathLibrary.MapRangeClamped` (.z _returnvalue) -360.0 360.0 -1.0 1.0))
    (set `self.Y-RotationRate` (`KismetMathLibrary.MapRangeClamped` (.y (`KismetMathLibrary.InverseTransformDirection` (`Actor.GetTransform` (`self.Character`)) _returnvalue)) -360.0 360.0 1.0 -1.0))
    (if (or (`self.DodgingLeft`) (`self.DodgingRight`))
      (`CharacterMovementComponent.AddForce` (`self.MovementComponent`) (* (select `bool` (`self.DodgingLeft`) :`false` _returnvalue_2 :`true` (* _returnvalue_2 -1.0)) (`self.DodgeCurrentForce`)))
      (set `self.DodgeCurrentForce` (`KismetMathLibrary.FInterpTo` (`self.DodgeCurrentForce`) 0.0 (`self.Delta`) 4.0)))
    (elif (!= _returnvalue_pitch 0.0)
      (`Actor.K2_SetActorRotation` (`self.Character`) (`KismetMathLibrary.RInterpTo` (`KismetMathLibrary.MakeRotator` _returnvalue_roll _returnvalue_pitch _returnvalue_yaw) (`KismetMathLibrary.MakeRotator` _returnvalue_roll 0.0 _returnvalue_yaw) (`self.Delta`) 8.0) false))))

(event `DodgeLeft`
  ;[0.599 1 0.6833] Left Dodge - set current dodge force equal to the default dodge force (applied during FlightUpdates). Dodge state ends after 1.5s. The 0.1s delay for the DoOnce ensures the AnimBP State machine moves out of the dodge state before being able to re-enter it.
  (if (`self.FastFlight`)
    (if (`KismetMathLibrary.BooleanNOR` (`self.DodgingLeft`) (`self.DodgingRight`))
      (`/Engine/EditorBlueprintResources/StandardMacros.DoOnce` false :!label _label_3
        (:`Completed`
          (set `self.DodgingLeft` true)
          (set `self.DodgeCurrentForce` (`self.DodgeDefaultForce`))
          (`KismetSystemLibrary.Delay` 1.5)
          (set `self.DodgingLeft` false)
          (`KismetSystemLibrary.Delay` 0.1)
          (goto _label_3 :!via `Reset`))))))

(event `DodgeRight`
  ;[0.599 1 0.6833] Right Dodge - set current dodge force equal to the default dodge force (applied during FlightUpdates). Dodge state ends after 1.5s. The 0.1s delay for the DoOnce ensures the AnimBP State machine moves out of the dodge state before being able to re-enter it.
  (if (`self.FastFlight`)
    (if (`KismetMathLibrary.BooleanNOR` (`self.DodgingLeft`) (`self.DodgingRight`))
      (`/Engine/EditorBlueprintResources/StandardMacros.DoOnce` false :!label _label_4
        (:`Completed`
          (set `self.DodgingRight` true)
          (set `self.DodgeCurrentForce` (`self.DodgeDefaultForce`))
          (`KismetSystemLibrary.Delay` 1.5)
          (set `self.DodgingRight` false)
          (`KismetSystemLibrary.Delay` 0.1)
          (goto _label_4 :!via `Reset`))))))

(event `MoveUp`
  (params (AxisValue :type "Float (double-precision)"))
  ;[0.599 1 0.6833] Handle input for hovering up and down
  (if (`self.Hover`)
    (`Pawn.AddMovementInput` (`self.Character`) (0.0 0.0 1.0) AxisValue false)))

(event `UpdateFastFlightSpeedUpdate`
  (set `CharacterMovementComponent.MaxAcceleration` 0.0 (`self.MovementComponent`))
  (`KismetSystemLibrary.Delay` 0.5)
  (if (`.bIsFlight` (`self.Check Is Flying`))
    (set `CharacterMovementComponent.MaxAcceleration` (`self.FastFlightAcceleration`) (`self.MovementComponent`))
    (`Camera.ChangeBlar` (`PlayerCharacter.Camera` (cast `/Game/_Users/Players/Blueprints/BP_PlayerBase` (`self.Character`) :!pure true)) true)))

(fn `Check Is Flying`
  (returns (bSuccess :type Boolean) (bIsHover :type Boolean) (bIsFlight :type Boolean))
  (bind _fastflight (`self.FastFlight`))
  (bind _hover (`self.Hover`))
  (return (or _hover _fastflight) _hover _fastflight))

(fn `ToggleFastFlight`
  (bind _character (`self.Character`))
  (bind _returnvalue (`KismetMathLibrary.MakeVector` (.x (`SceneComponent.K2_GetComponentLocation` (`self.CapsuleComponent`))) (.y (`SceneComponent.K2_GetComponentLocation` (`self.CapsuleComponent`))) (+ (- (.z (`SceneComponent.K2_GetComponentLocation` (`self.CapsuleComponent`))) (`self.CapsuleHalfHeight`)) (`self.CapsuleRadius`))))
  (bind _returnvalue_2 (`KismetMathLibrary.MakeVector` (.x (`SceneComponent.K2_GetComponentLocation` (`self.CapsuleComponent`))) (.y (`SceneComponent.K2_GetComponentLocation` (`self.CapsuleComponent`))) (- (+ (.z (`SceneComponent.K2_GetComponentLocation` (`self.CapsuleComponent`))) (`self.CapsuleHalfHeight`)) (`self.CapsuleRadius`))))
  (if (not (`self.GroundSlam`))
    (bind _output_get (set `self.FastFlight` (not (`self.FastFlight`))))
    (if _output_get
      (if (`self.Hover`)
        (`self.ToggleHover`)
        (else
          (`PlayerCharacter.ChangePlayerMode` (cast `/Game/_Users/Players/Blueprints/BP_Player` (`self.Character`) :!pure true) (enumliteral `EPlayerModeType` "Statue") false)))
      (`Actor.K2_SetActorRotation` _character (`Actor.K2_GetActorRotation` (`PlayerCharacter.Camera` (cast `/Game/_Users/Players/Blueprints/BP_PlayerBase` _character :!pure true))) false)
      ;[1 1 1] 速度、加速度を変更
      (set `CharacterMovementComponent.MaxFlySpeed` (`self.FastFlightSpeed`) (`self.MovementComponent`))
      (`self.UpdateFastFlightSpeedUpdate`)
      ;[1 1 1] Characterの移動モードを更新
      (`CharacterMovementComponent.SetMovementMode` (`self.MovementComponent`) "MOVE_Flying" 0)
      (set `CharacterMovementComponent.bOrientRotationToMovement` true (`self.MovementComponent`))
      ;[1 1 1] カプセルコリジョンの大きさを調整
      (`CapsuleComponent.SetCapsuleHalfHeight` (`self.CapsuleComponent`) (`CapsuleComponent.GetUnscaledCapsuleRadius` (`self.CapsuleComponent`)) true)
      (set `self.CurrentMaxFlySpeed` (`CharacterMovementComponent.MaxFlySpeed` (`self.MovementComponent`)))
      (else
        (`Camera.ChangeBlar` (`PlayerCharacter.Camera` (cast `/Game/_Users/Players/Blueprints/BP_PlayerBase` (`self.Character`) :!pure true)) false)
        ;[1 1 1] カプセルコリジョンのサイズを戻していいか確認し、ダメならFastFlight続行
        (bind (_outhit _returnvalue_3) (`KismetSystemLibrary.CapsuleTraceSingle` _returnvalue_2 (+ _returnvalue_2 (0.01 0.01 0.01)) (`self.CapsuleRadius`) (`self.CapsuleHalfHeight`) "TraceTypeQuery1"))
        (if _returnvalue_3
          (bind (_outhit_2 _returnvalue_4) (`KismetSystemLibrary.CapsuleTraceSingle` _returnvalue (- _returnvalue (0.01 0.01 0.01)) (`self.CapsuleRadius`) (`self.CapsuleHalfHeight`) "TraceTypeQuery1"))
          (if _returnvalue_4
            (set `self.FastFlight` true)
            (else
              ;[1 1 1] Z方向の速度量を取得
              (bind _returnvalue_5 (`PrimitiveComponent.GetPhysicsLinearVelocity` (`self.CapsuleComponent`) "None" :!label _label))
              (set `self.Z-Momentum` (.z _returnvalue_5))
              (`CharacterMovementComponent.SetMovementMode` (`self.MovementComponent`) "MOVE_Walking" 0)
              (set `CharacterMovementComponent.bOrientRotationToMovement` false (`self.MovementComponent`))
              (`CapsuleComponent.SetCapsuleHalfHeight` (`self.CapsuleComponent`) (`self.CapsuleHalfHeight`) true)
              ;[1 1 1] 回避をキャンセル
              (set `self.DodgingLeft` false)
              (set `self.DodgingRight` false)
              ;[1 1 1] どちらの飛行モードでも無くなったなら、Z方向の勢いをある程度与える
              (if (`KismetMathLibrary.BooleanNOR` (`self.Hover`) (`self.FastFlight`))
                (`Character.LaunchCharacter` (`self.Character`) (`KismetMathLibrary.MakeVector` 0.0 0.0 (* (`self.Z-Momentum`) 0.7)) false true)
                (`/Game/_Users/Players/Blueprints/BP_Player.ChangePlayerMode` (cast `/Game/_Users/Players/Blueprints/BP_Player` (`self.Character`) :!pure true) (enumliteral `EPlayerModeType` "Human") false))))
          (else
            (goto _label)))))))

(fn `ToggleHover`
  (if (not (`self.GroundSlam`))
    (bind _output_get (set `self.Hover` (not (`self.Hover`))))
    (if _output_get
      (if (`self.FastFlight`)
        (`self.ToggleFastFlight`)
        (else
          (`/Game/_Users/Players/Blueprints/BP_Player.ChangePlayerMode` (cast `/Game/_Users/Players/Blueprints/BP_Player` (`self.Character`) :!pure true) (enumliteral `EPlayerModeType` "Statue") false)))
      (if (`self.FastFlight`)
        (set `self.Hover` false)
        (else
          (set `CharacterMovementComponent.MaxFlySpeed` (`self.HoverSpeed`) (`self.MovementComponent`))
          (set `CharacterMovementComponent.MaxAcceleration` (`self.DefaultAcceleration`) (`self.MovementComponent`))
          (`CharacterMovementComponent.SetMovementMode` (`self.MovementComponent`) "MOVE_Flying" 0)
          (set `CharacterMovementComponent.bOrientRotationToMovement` false (`self.MovementComponent`))
          (set `self.CurrentMaxFlySpeed` (`CharacterMovementComponent.MaxFlySpeed` (`self.MovementComponent`)))))
      (else
        (bind _returnvalue (`PrimitiveComponent.GetPhysicsLinearVelocity` (`self.CapsuleComponent`) "None"))
        (set `self.Z-Momentum` (.z _returnvalue))
        (`CharacterMovementComponent.SetMovementMode` (`self.MovementComponent`) "MOVE_Walking" 0)
        (set `CharacterMovementComponent.bOrientRotationToMovement` true (`self.MovementComponent`))
        (if (`KismetMathLibrary.BooleanNOR` (`self.Hover`) (`self.FastFlight`))
          (`Character.LaunchCharacter` (`self.Character`) (`KismetMathLibrary.MakeVector` 0.0 0.0 (* (`self.Z-Momentum`) 0.7)) false true)
          (`/Game/_Users/Players/Blueprints/BP_Player.ChangePlayerMode` (cast `/Game/_Users/Players/Blueprints/BP_Player` (`self.Character`) :!pure true) (enumliteral `EPlayerModeType` "Human") false))))))

(fn `TriggerGroundSlam`
  (set `self.GroundSlam` true)
  (`Controller.SetIgnoreMoveInput` (`Pawn.GetController` (`self.Character`)) true)
  (`/Game/_Users/Players/Blueprints/BP_Player.ChangePlayerMode` (cast `/Game/_Users/Players/Blueprints/BP_Player` (`self.Character`) :!pure true) (enumliteral `EPlayerModeType` "Human") true))