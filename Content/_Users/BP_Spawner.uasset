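; BP_Spawner builds a grid of NewBlueprint actors from its root location at BeginPlay, shifting alternate rows by a fixed Y offset.
; Each row is a loop that chains spawns through the previous actor's left location.
; A further actor spawned at the stored front location seeds the next row, and Redraw calls itself until the counter passes Columb.
; Spawn locations are printed for debugging.
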(event `Redraw`
  (bind _next (`self.Next`))
  (bind _front (`self.Front`))
  (for _ (range (+ (`self.Row`) 1)) :!label _label
    (bind _returnvalue (`|SpawnActorFromClass` "/Game/NewBlueprint.NewBlueprint_C" (`KismetMathLibrary.MakeTransform` _next (struct) (`self.Scale`)) "Undefined" "OverrideRootScale" null null))
    (`KismetSystemLibrary.PrintString` (`KismetStringLibrary.Conv_VectorToString` _next))
    (set `self.Next` (`TestCube.GetLeftLocation` _returnvalue))
    (`/Engine/EditorBlueprintResources/StandardMacros.DoOnce` false
      (:`Completed`
        (set `self.Front` (`TestCube.GetFrontLocation` _returnvalue)))))
  (bind _returnvalue_2 (`|SpawnActorFromClass` "/Game/NewBlueprint.NewBlueprint_C" (`KismetMathLibrary.MakeTransform` _front (struct) (`self.Scale`)) "Undefined" "OverrideRootScale" null null))
  (`KismetSystemLibrary.PrintString` (`KismetStringLibrary.Conv_VectorToString` _front))
  (set `self.Next` (`TestCube.GetLeftLocation` _returnvalue_2))
  (set `self.Front` (`TestCube.GetFrontLocation` _returnvalue_2))
  (if (<= (`self.Count`) (`self.Columb`))
    (`/Engine/EditorBlueprintResources/StandardMacros.IncrementInt` (`self.Count`)
      (:`  `
        (if (== (mod (`self.Count`) 2) 0)
          (set `self.Next` (+ (`self.Next`) (0.0 -25.0 0.0))))
        (`self.Redraw`)))))

(event `self.ReceiveBeginPlay`
  (set `self.Next` (`SceneComponent.K2_GetComponentLocation` (`self.DefaultSceneRoot`)))
  (goto _label))

(fn `UserConstructionScript`)