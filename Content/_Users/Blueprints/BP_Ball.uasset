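; Grabbable, throwable ball actor that switches between Grab, Physics and Fly modes, each configuring simulation and collision.
; Overlapping a player whose BPGrab accepts it attaches the ball there and binds Throw to the component's throw event.
; Throw returns it to Physics and stores a direction toward the player's throw target.
; Leaving Grab detaches it and delays re-enabling pickup collision; physics-mode hits call Bound.
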(event `self.Sphere.OnComponentHit`
  (params (HitComponent :type "PrimitiveComponent Object Reference") (OtherActor :type "Actor Object Reference") (OtherComp :type "PrimitiveComponent Object Reference") (NormalImpulse :type "Vector Structure") (Hit :type "HitResult Structure (by ref)"))
  (switch `EBallMoveType` (`self.nowType`)
    (:`Physics`
      (`self.Bound` NormalImpulse))))

(event `self.Col.OnComponentBeginOverlap`
  (params (OverlappedComponent :type "PrimitiveComponent Object Reference") (OtherActor :type "Actor Object Reference") (OtherComp :type "PrimitiveComponent Object Reference") (OtherBodyIndex :type Integer) (bFromSweep :type Boolean) (SweepResult :type "HitResult Structure (by ref)"))
  (bind _asbp_player (cast `/Game/_Users/Players/Blueprints/BP_Player` OtherActor))
  (bind _bp_grab (`/Game/_Users/Players/Blueprints/BP_Player.BP_Grab` _asbp_player))
  (if (`/Game/_Users/Blueprints/BP_Grab.SetBall` _bp_grab self)
    (add `/Game/_Users/Blueprints/BP_Grab.Throw` _bp_grab (delegate `Throw`))
    (set `self.NowGrabComponent` _bp_grab)
    (`self.ChangeMode` "Grab")
    (`self.K2_AttachToComponent` _bp_grab "None" "SnapToTarget" "SnapToTarget" "KeepRelative")))

(event `Throw`
  (remove `/Game/_Users/Blueprints/BP_Grab.Throw` (`self.NowGrabComponent`) (delegate `Throw`))
  (`self.ChangeMode` "Physics")
  (set `self.Dir` (`KismetMathLibrary.Conv_RotatorToVector` (`KismetMathLibrary.FindLookAtRotation` (`self.K2_GetActorLocation`) (`/Game/_Users/Players/Blueprints/BP_Player.GetThrowTarget` (cast `/Game/_Users/Players/Blueprints/BP_Player` (`ActorComponent.GetOwner` (`self.NowGrabComponent`)) :!pure true))))))

(event `Invincible`
  (`KismetSystemLibrary.Delay` (`self.InvincibleDelayTime`))
  (`PrimitiveComponent.SetCollisionEnabled` (`self.Col`) "QueryOnly"))

(fn `ChangeMode`
  (params (newType :type "EBallMoveType Enum" :default "Grab"))
  (if (`|EnumInequality` newType (`self.NowType`))
    (`self.EndMode`)
    (set `self.NowType` (`local.newType`))
    (`self.InitMode`)))

(fn `EndMode`
  (switch `EBallMoveType` (`self.NowType`)
    (:`Grab`
      (`self.K2_DetachFromActor` "KeepWorld" "KeepWorld" "KeepWorld")
      (`self.Invincible`))))

(fn `InitMode`
  (switch `EBallMoveType` (`self.NowType`)
    (:`Grab`
      (`PrimitiveComponent.SetSimulatePhysics` (`self.Sphere`) false)
      (`PrimitiveComponent.SetCollisionEnabled` (`self.Sphere`) "NoCollision")
      (`PrimitiveComponent.SetCollisionEnabled` (`self.Col`) "NoCollision"))
    (:`Physics`
      (`PrimitiveComponent.SetSimulatePhysics` (`self.Sphere`) true)
      (`PrimitiveComponent.SetCollisionEnabled` (`self.Sphere`) "QueryAndPhysics"))
    (:`Fly`
      (`PrimitiveComponent.SetSimulatePhysics` (`self.Sphere`) false)
      (`PrimitiveComponent.SetCollisionEnabled` (`self.Sphere`) "QueryAndPhysics"))))

(fn `UserConstructionScript`)