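; BP_Grab is a component that lets its owning Character hold and throw one ball.
; On BeginPlay it attaches to the "grab" socket on the character's mesh.
; SetBall stores a ball reference only when none is held, and IsGrabbing reports whether one is held.
; ThrowBall passes a new speed to the held ball, sets an IsThrow flag and clears the reference.
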(event `self.ReceiveBeginPlay`
  (`self.K2_AttachToComponent` (`Character.Mesh` (cast `Character` (`self.GetOwner`) :!pure true)) "grab" "KeepRelative" "KeepRelative" "KeepRelative"))

(fn `IsGrabbing`
  (returns (Return :type Boolean))
  (return (`KismetSystemLibrary.IsValid` (`self.Ball`))))

(fn `SetBall`
  (params (NewBall :type "/Game/_Users/Blueprints/BP_Ball Object Reference"))
  (returns (Success :type Boolean))
  (`/Engine/EditorBlueprintResources/StandardMacros.IsValid` (`self.Ball`)
    (:`Is Valid`
      (return false))
    (:`Is Not Valid`
      (set `self.Ball` (`local.NewBall`))
      (return true))))

(fn `ThrowBall`
  (params (NewSpeed :type "Float (double-precision)"))
  (`/Engine/EditorBlueprintResources/StandardMacros.IsValid` (`self.Ball`)
    (:`Is Valid`
      (set `Ball.Speed` (`local.NewSpeed`) (`self.Ball`))
      (set `self.bIsThrow` true)
      (set `self.Ball` null))))