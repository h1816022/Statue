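; BP_Camera is a camera actor, derived from a parent camera Blueprint, that follows the player's control rotation.
; On BeginPlay it hands its CameraComponent to the player's BP_DynamicFlightComponent, then calls ChangeBlar on and off on timed delays.
; UpdateTransform extends the parent by snapping actor rotation to control rotation.
; The flying check there has empty branches, and an interpolated rotation alternative is left unconnected.
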(event `self.ReceiveBeginPlay`
  (`parent.ReceiveBeginPlay`)
  (set `/Game/DynamicFlight/Blueprints/Components/BP_DynamicFlightComponent.CameraComponent` (`self.GetCameraComponent`) (`self.GetComponentByClass` (`self.Player`) "/Game/DynamicFlight/Blueprints/Components/BP_DynamicFlightComponent.BP_DynamicFlightComponent_C"))
  (`KismetSystemLibrary.Delay` 5.0)
  (`self.ChangeBlar` true)
  (`KismetSystemLibrary.Delay` 5.0)
  (`self.ChangeBlar` false))

(event `self.UpdateTransform`
  (`parent.UpdateTransform`)
  (bind _dynamicflightcomponent (message `/Game/DynamicFlight/Blueprints/Interfaces/DynamicFlightInterface.GetDynamicFlightComponent` (`self.Player`)))
  (if (`.bIsFlying` (`/Game/DynamicFlight/Blueprints/Components/BP_DynamicFlightComponent.CheckIsFlying` _dynamicflightcomponent))
    _
    (else
      _))
  (`self.K2_SetActorRotation` (`Pawn.GetControlRotation` (`self.Player`))))

(fn `UserConstructionScript`)