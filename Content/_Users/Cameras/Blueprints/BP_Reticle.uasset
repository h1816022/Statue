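; Actor that creates a screen reticle widget and scales it by the distance to what the camera is aimed at.
; Each tick a visibility trace runs forward from the referenced camera, ignoring the player pawn, and enlarges the reticle image as hits get closer.
; It stores the impact point, or the trace end on a miss, in TargetPos and rotates itself to face the camera.
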(event `self.ReceiveBeginPlay`
  (bind _returnvalue (`|CreateWidget` "/Game/_Users/Cameras/Widgets/WBP_Reticle.WBP_Reticle_C"))
  (bind _output_get (set `self.Reticle` _returnvalue))
  (`UserWidget.AddToViewport` _output_get 0))

(event `self.ReceiveTick`
  (params (DeltaSeconds :type "Float (single-precision)"))
  (bind _camera (`Camera.Camera` (`self.Camera`)))
  (bind _returnvalue (`SceneComponent.K2_GetComponentLocation` _camera))
  (bind _returnvalue_2 (+ _returnvalue (* (`SceneComponent.GetForwardVector` _camera) (`self.TraceLength`))))
  (bind _outhit (`KismetSystemLibrary.LineTraceSingle` _returnvalue _returnvalue_2 "TraceTypeQuery1" false (`|MakeArray` (`GameplayStatics.GetPlayerPawn` 0) :!type "Actor Object Reference")))
  (if (`GameplayStatics.BreakHitResult` _outhit)
    (bind _returnvalue_3 (`KismetMathLibrary.Lerp` (`self.MaxScale`) 1.0 (/ (`.Distance` (`GameplayStatics.BreakHitResult` _outhit)) (`self.TraceLength`))))
    (`Widget.SetRenderScale` (`/Game/_Users/Cameras/Widgets/WBP_Reticle.Image_123` (`self.Reticle`)) (`KismetMathLibrary.MakeVector2D` _returnvalue_3 _returnvalue_3))
    (set `self.TargetPos` (`.ImpactPoint` (`GameplayStatics.BreakHitResult` _outhit)))
    (else
      (`Widget.SetRenderScale` (`/Game/_Users/Cameras/Widgets/WBP_Reticle.Image_123` (`self.Reticle`)) (1.0 1.0))
      (set `self.TargetPos` _returnvalue_2)))
  (`self.K2_SetActorRotation` (`KismetMathLibrary.FindLookAtRotation` (`self.K2_GetActorLocation`) (`SceneComponent.K2_GetComponentLocation` (`Camera.Camera` (`self.Camera`))))))

(fn `UserConstructionScript`)