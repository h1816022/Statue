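; BP_NeoCube is a cube actor that extends inherited movement behavior with a timed motion sequence.
; On BeginPlay it runs the parent logic and turns moving on, then switches moving off twelve seconds later.
; In parallel, after a five-second delay, a zero-delay loop acts as a per-frame tick, steadily growing MaxDistance by scaled delta time with no exit condition.
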(event `self.ReceiveBeginPlay`
  (`parent.ReceiveBeginPlay`)
  (`|ExecutionSequence`
    (:`then_0`
      (`self.SetIsMoving` true)
      (`KismetSystemLibrary.Delay` 5.0)
      (set `self.MaxDistance` (+ (`self.MaxDistance`) (* (`GameplayStatics.GetWorldDeltaSeconds`) 150.0)) :!label _label)
      (`KismetSystemLibrary.Delay` 0.0)
      (goto _label))
    (:`then_1`
      (`KismetSystemLibrary.Delay` 12.0)
      (`self.SetIsMoving` false))))

(fn `UserConstructionScript`)