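; BP_Spawner is an actor that lays out a staggered grid of BP_NeoCube actors from its root location at BeginPlay.
; A loop spawns Row-driven lines of cubes along negative Y, with a DoOnce capturing the first Front anchor.
; After each line, a cube spawned at Front starts the next one and advances the anchor along X.
; Redraw calls itself recursively until Count passes Columb, adding a Y offset on even counts.
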(event `Redraw`
  (for _ (range (+ (`self.Row`) 1)) :!label _label
    (bind _returnvalue (`|SpawnActorFromClass` "/Game/_Users/Cubes/BP_NeoCube.BP_NeoCube_C" (`KismetMathLibrary.MakeTransform` (`self.Next`) (struct) (`self.Scale`)) "Undefined" "OverrideRootScale" null null))
    (bind _returnvalue_2 (`self.K2_GetActorLocation` _returnvalue))
    (set `self.Next` (+ _returnvalue_2 (0.0 -100.0 0.0)))
    (`/Engine/EditorBlueprintResources/StandardMacros.DoOnce` false
      (:`Completed`
        (set `self.Front` (+ _returnvalue_2 (50.0 0.0 0.0))))))
  (bind _returnvalue_3 (`|SpawnActorFromClass` "/Game/_Users/Cubes/BP_NeoCube.BP_NeoCube_C" (`KismetMathLibrary.MakeTransform` (`self.Front`) (struct) (`self.Scale`)) "Undefined" "OverrideRootScale" null null))
  (bind _returnvalue_4 (`self.K2_GetActorLocation` _returnvalue_3))
  (set `self.Next` (+ _returnvalue_4 (0.0 -100.0 0.0)))
  (set `self.Front` (+ _returnvalue_4 (50.0 0.0 0.0)))
  (if (<= (`self.Count`) (`self.Columb`))
    (`/Engine/EditorBlueprintResources/StandardMacros.IncrementInt` (`self.Count`)
      (:`  `
        (if (== (mod (`self.Count`) 2) 0)
          (set `self.Next` (+ (`self.Next`) (0.0 -25.0 0.0))))
        (`self.Redraw`)))))

(event `self.ReceiveBeginPlay`
  (set `self.Next` (`SceneComponent.K2_GetComponentLocation` (`self.DefaultSceneRoot`)))
  (goto _label))

(fn `UserConstructionScript`)