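; BP_Camera is a player camera actor that adapts its rotation to whether the player is flying.
; On BeginPlay it hands its camera component to the player's BP_DynamicFlightComponent.
; Each transform update queries that component's flying state after running the parent logic.
; In flight, rotation eases toward the velocity direction with a fixed-alpha lerp; otherwise it snaps to control rotation.
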(event `self.ReceiveBeginPlay`
  (`parent.ReceiveBeginPlay`)
  (set `/Game/DynamicFlight/Blueprints/Components/BP_DynamicFlightComponent.CameraComponent` (`self.GetCameraComponent`) (`self.GetComponentByClass` (`self.Player`) "/Game/DynamicFlight/Blueprints/Components/BP_DynamicFlightComponent.BP_DynamicFlightComponent_C")))

(event `self.UpdateTransform`
  (`parent.UpdateTransform`)
  (bind _dynamicflightcomponent (message `/Game/DynamicFlight/Blueprints/Interfaces/DynamicFlightInterface.GetDynamicFlightComponent` (`self.Player`)))
  (if (`.bIsFlying` (`/Game/DynamicFlight/Blueprints/Components/BP_DynamicFlightComponent.CheckIsFlying` _dynamicflightcomponent))
    (`self.K2_SetActorRotation` (`KismetMathLibrary.RLerp` (`self.K2_GetActorRotation`) (`KismetMathLibrary.Conv_VectorToRotator` (`self.GetVelocity` (`self.Player`))) 0.01))
    (else
      (`self.K2_SetActorRotation` (`Pawn.GetControlRotation` (`self.Player`))))))

(fn `UserConstructionScript`)