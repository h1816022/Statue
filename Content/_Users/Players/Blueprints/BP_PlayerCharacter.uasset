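; Player character Blueprint that lets the player switch between a default and a statue mode with the Q key.
; At BeginPlay it creates a dynamic material instance from the mesh's first material.
; ChangeMode plays a timeline forward for Statue or in reverse otherwise, driving the material's DissolveRate parameter.
; A CanChangeMode flag blocks further switches until the timeline finishes and commits the new mode.
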(event `self.ReceiveBeginPlay`
  (bind _mesh (`self.Mesh`))
  (`parent.ReceiveBeginPlay`)
  (bind _returnvalue (`PrimitiveComponent.CreateDynamicMaterialInstance` _mesh 0 (`PrimitiveComponent.GetMaterial` _mesh 0) "None"))
  (set `self.Material` _returnvalue))

(event `ChangeMode`
  (params (NewType :type "EPlayerModeType Enum" :default "Default"))
  (if (`self.bCanChangeMode`)
    (if (`|EnumInequality` (`self.NowModeType`) NewType)
      (set `self.bCanChangeMode` false)
      (switch `EPlayerModeType` NewType
        (:`Default`
          (bind (_direction _newtrack_0) (`Timeline|Timeline_0` :!via `ReverseFromEnd` :!label _label)
            (:`Update`
              (`MaterialInstanceDynamic.SetScalarParameterValue` (`self.Material`) "DissolveRate" _newtrack_0))
            (:`Finished`
              (set `self.NowModeType` NewType)
              (set `self.bCanChangeMode` true))))
        (:`Statue`
          (goto _label :!via `PlayFromStart`))))))

(event `Key|Q`
  (params (Key :type "Key Structure"))
  (:`Pressed`
    (switch `EPlayerModeType` (`self.NowModeType`)
      (:`Default`
        (`self.ChangeMode` "Statue"))
      (:`Statue`
        (`self.ChangeMode` "Default")))))

(fn `UserConstructionScript`)