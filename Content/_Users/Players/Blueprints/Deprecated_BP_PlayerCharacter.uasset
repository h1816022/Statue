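; Deprecated player character Blueprint that toggles between Default and Statue modes and tracks locomotion state.
; Q triggers the mode change, which drives a dissolve timeline on a dynamic mesh material and blocks further switches until it finishes.
; Tick derives rotation rate, movement, acceleration and speed values, capturing the speed at the moment acceleration stops.
; Walk and Sprint inputs set a target speed that Tick smoothly interpolates MaxWalkSpeed toward.
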(event `self.ReceiveBeginPlay`
  (bind _mesh (`self.Mesh`))
  (`parent.ReceiveBeginPlay`)
  (bind _returnvalue (`PrimitiveComponent.CreateDynamicMaterialInstance` _mesh 0 (`PrimitiveComponent.GetMaterial` _mesh 0) "None"))
  (set `self.Material` _returnvalue))

(event `ChangeMode`
  (params (NewType :type "EPlayerModeType Enum" :default "Default"))
  (if (`self.bCanChangeMode`)
    (if (`|EnumInequality` (`self.NowModeType`) NewType)
      (set `self.bCanChangeMode` false)
      (switch `EPlayerModeType` NewType
        (:`Default`
          (bind (_direction _newtrack_0) (`Timeline|Timeline_0` :!via `ReverseFromEnd` :!label _label)
            (:`Update`
              (`MaterialInstanceDynamic.SetScalarParameterValue` (`self.Material`) "DissolveRate" _newtrack_0))
            (:`Finished`
              (set `self.NowModeType` NewType)
              (set `self.bCanChangeMode` true))))
        (:`Statue`
          (goto _label :!via `PlayFromStart`))))))

(event `Key|Q`
  (params (Key :type "Key Structure"))
  (:`Pressed`
    (switch `EPlayerModeType` (`self.NowModeType`)
      (:`Default`
        (`self.ChangeMode` "Statue"))
      (:`Statue`
        (`self.ChangeMode` "Default")))))

(event `self.ReceiveTick`
  (params (DeltaSeconds :type "Float (single-precision)"))
  (bind _returnvalue (`self.GetVelocity`))
  (bind (_returnvalue_x _returnvalue_y _returnvalue_z) (`KismetMathLibrary.BreakVector` (`PrimitiveComponent.GetPhysicsAngularVelocityInDegrees` (`self.CapsuleComponent`) "None")))
  (set `self.Delta` DeltaSeconds)
  (set `self.CurrentRotationRate` (`KismetMathLibrary.MapRangeClamped` _returnvalue_z -360.0 360.0 -1.0 1.0))
  (set `self.bIsMoving` (!= (`SceneComponent.GetComponentVelocity` (`self.CapsuleComponent`)) (0.0 0.0 0.0)))
  (bind _output_get (set `self.bIsAccelerating` (> (`KismetMathLibrary.VSize` (`CharacterMovementComponent.GetCurrentAcceleration` (`self.CharacterMovement`))) 0.0)))
  (if _output_get
    (goto _label_2 :!via `Reset In`)
    (else
      (`|ExecutionSequence`
        (:`then_0`
          (`|DoOnceMultiInput` :!label _label_2
            (:`A Out`
              (set `self.SpeedWhenStopping` (`self.CurrentSpeed`)))
            (:`Reset Out`
              (set `self.CurrentSpeed` (`KismetMathLibrary.VSize` _returnvalue) :!label _label_3)
              (set `self.Lateralspeed` (`KismetMathLibrary.VSizeXY` _returnvalue))
              (set `CharacterMovementComponent.MaxWalkSpeed` (`KismetMathLibrary.FInterpTo` (`CharacterMovementComponent.MaxWalkSpeed` (`self.CharacterMovement`)) (`self.MaxSpeedTarget`) (`self.Delta`) 4.0) (`self.CharacterMovement`)))))
        (:`then_1`
          (goto _label_3))))))

(event `InputAction|Walk`
  (params (Key :type "Key Structure"))
  (:`Pressed`
    (set `self.MaxSpeedTarget` (`self.WalkSpeed`)))
  (:`Released`
    (set `self.MaxSpeedTarget` (`self.JogSpeed`))))

(event `InputAction|Sprint`
  (params (Key :type "Key Structure"))
  (:`Pressed`
    (set `self.MaxSpeedTarget` (`self.RunSpeed`)))
  (:`Released`
    (set `self.MaxSpeedTarget` (`self.JogSpeed`))))

(fn `UserConstructionScript`)